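; Actor Blueprint that spins itself around the bounds center of its MpcPivotDataWheel component.
; Each Tick it chains three rotations, an X tilt, a half-turn about Z and the opposite tilt, to turn about a slightly tilted axis without delta-time scaling.
; A helper function rotates both location and orientation around the given point and axis.
; A time-based SetActorRotation spin is left unconnected.
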(event `self.ReceiveBeginPlay`)

(event `self.ReceiveTick`
  (params (DeltaSeconds :type "Float (single-precision)"))
  (bind _origin (`KismetSystemLibrary.GetComponentBounds` (`self.mpc_PivotDataWheel`)))
  (`self.RotateActorAroundPoint` 5.11989 _origin)
  (`self.RotateActorAroundPoint` 180.0 _origin (0.0 0.0 1.0))
  (`self.RotateActorAroundPoint` -5.11989 _origin))

(fn `RotateActorAroundPoint`
  (params (AngleDeg :type "Float (double-precision)" :default 1.0) (`Point to Rotate Around` :type "Vector Structure") (`Axis to Rotate Around` :type "Vector Structure" :default (1.0 0.0 0.0)))
  (`self.K2_SetActorLocationAndRotation` (+ (`KismetMathLibrary.RotateAngleAxis` (- (`self.K2_GetActorLocation`) `Point to Rotate Around`) AngleDeg `Axis to Rotate Around`) `Point to Rotate Around`) (`KismetMathLibrary.ComposeRotators` (`self.K2_GetActorRotation`) (`KismetMathLibrary.RotatorFromAxisAndAngle` `Axis to Rotate Around` AngleDeg))))

(fn `UserConstructionScript`)